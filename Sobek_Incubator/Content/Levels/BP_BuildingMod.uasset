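; BP_BuildingMod is a procedural building Blueprint that tiles one wall mesh into a flat grid along X and Z.
; The construction script derives tile size from the MeshWall bounds, then nested loops over BuildingHeight and BuildingWidth add an offset static mesh component per cell.
; All logic runs at construction; the event graph holds only disabled default events.
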(event EventBeginPlay)

(event Collision|EventActorBeginOverlap
  (params (OtherActor :type Actor%20Object%20Reference)))

(event EventTick
  (params (DeltaSeconds :type Float%20%28single-precision%29)))

(fn ConstructionScript
  (bind _mesh_wall (Variables|Default|GetMesh%20Wall))
  (bind _returnvalue (StaticMesh|GetBounds _mesh_wall))
  (bind (_x _y _z) (Math|Vector|BreakVector (.boxextent _returnvalue)))
  (Utilities|FlowControl|Sequence
    (:then_0
      (LocalVariables|SetMesh%20Width (* _x 2.0))
      (LocalVariables|SetMesh%20Height (* _z 2.0)))
    (:then_1
      (for _index (range 0 (- (Variables|Default|GetBuilding%20Height) 1))
        (for _index_2 (range 0 (- (Variables|Default|GetBuilding%20Width) 1))
          (bind _returnvalue_2 (AddComponent|AddStaticMeshComponent false (Math|Transform|MakeTransform (Math|Vector|MakeVector (* _index_2 (LocalVariables|GetMesh%20Width)) 0.0 (* _index (LocalVariables|GetMesh%20Height))))))
          (Components|StaticMesh|SetStaticMesh _returnvalue_2 (Variables|Default|GetMesh%20Wall)))))))