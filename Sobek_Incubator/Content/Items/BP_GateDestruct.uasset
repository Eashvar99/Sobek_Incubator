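; Destructible double physics gate that breaks open when an overlapping ToolCart holds three items and is not available.
; Breaking releases both physics constraints and clears angular damping on each half.
; When either half next wakes, the gate plays a break sound once and kicks the halves with opposite angular impulses, then raises damping.
; Until broken, waking halves play hit sounds above a spin threshold, after a short BeginPlay grace delay.
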(event OnComponentWake(HalfGateLeft)
  (params (WakingComponent :type Primitive%20Component%20Object%20Reference) (BoneName :type Name :default "None"))
  (bind _halfgateleft (Variables|Default|GetHalfGateLeft))
  (bind _returnvalue (Physics|GetPhysicsAngularVelocityinDegrees _halfgateleft "None"))
  (if (Variables|Default|Getready)
    (Utilities|FlowControl|DoOnce false :!label _label
      (:Completed
        (if (Variables|Default|Getbroken)
          (Utilities|FlowControl|DoOnce false
            (:Completed
              (Audio|PlaySoundatLocation "/Game/Sound/Gate_Break.Gate_Break" (Transformation|GetWorldLocation (Variables|Default|GetDefaultSceneRoot)) "0, 0, 0" 0.5 1.0 0.0 0 0 0)
              (Class|PrimitiveComponent|AddAngularImpulseinDegrees (Variables|Default|GetHalfGateLeft) "0, 0,-80.000000" "None" true)
              (Class|PrimitiveComponent|AddAngularImpulseinDegrees (Variables|Default|GetHalfGateRight) "0, 0,80.000000" "None" true)
              (Utilities|FlowControl|Delay 1.0)
              (Class|PrimitiveComponent|SetAngularDamping (Variables|Default|GetHalfGateLeft) 1e+01)
              (Class|PrimitiveComponent|SetAngularDamping (Variables|Default|GetHalfGateRight) 1e+01)))
          (else
            (if (or (> (.z _returnvalue) 1.5) (< (.z _returnvalue) -1.5))
              (Audio|PlaySoundatLocation "/Game/Sound/GateHit_Cue.GateHit_Cue" (Transformation|GetWorldLocation WakingComponent) "0, 0, 0" 0.5 1.0 0.0 0 0 0))
            (Utilities|FlowControl|Delay 0.2)
            (goto _label Reset)))))))

(event OnComponentWake(HalfGateRight)
  (params (WakingComponent :type Primitive%20Component%20Object%20Reference) (BoneName :type Name :default "None"))
  (bind _halfgateright (Variables|Default|GetHalfGateRight))
  (bind _returnvalue (Physics|GetPhysicsAngularVelocityinDegrees _halfgateright "None"))
  (if (Variables|Default|Getready)
    (Utilities|FlowControl|DoOnce false :!label _label
      (:Completed
        (if (Variables|Default|Getbroken)
          (Utilities|FlowControl|DoOnce false
            (:Completed
              (Audio|PlaySoundatLocation "/Game/Sound/Gate_Break.Gate_Break" (Transformation|GetWorldLocation (Variables|Default|GetDefaultSceneRoot)) "0, 0, 0" 0.5 1.0 0.0 0 0 0)
              (Class|PrimitiveComponent|AddAngularImpulseinDegrees (Variables|Default|GetHalfGateLeft) "0, 0,-80.000000" "None" true)
              (Class|PrimitiveComponent|AddAngularImpulseinDegrees (Variables|Default|GetHalfGateRight) "0, 0,80.000000" "None" true)
              (Utilities|FlowControl|Delay 1.0)
              (Class|PrimitiveComponent|SetAngularDamping (Variables|Default|GetHalfGateLeft) 1e+01)
              (Class|PrimitiveComponent|SetAngularDamping (Variables|Default|GetHalfGateRight) 1e+01)))
          (else
            (if (or (> (.z _returnvalue) 1.5) (< (.z _returnvalue) -1.5))
              (Audio|PlaySoundatLocation "/Game/Sound/GateHit_Cue.GateHit_Cue" (Transformation|GetWorldLocation WakingComponent) "0, 0, 0" 0.5 1.0 0.0 0 0 0))
            (Utilities|FlowControl|Delay 0.2)
            (goto _label Reset)))))))

(event Collision|EventActorBeginOverlap
  (params (OtherActor :type Actor%20Object%20Reference))
  (if (Actor|ActorHasTag OtherActor "Toolcart")
    (bind _astool_cart (Utilities|Casting|CastToToolCart OtherActor))
    (if (== (Variables|/Game/Movables/ToolCart.ToolCart_C|GetItems _astool_cart) 3)
      (bind _astool_cart_2 (Utilities|Casting|CastToToolCart OtherActor))
      (if (not (Variables|/Game/Movables/ToolCart.ToolCart_C|GetisAvailable _astool_cart_2))
        (Utilities|FlowControl|DoOnce false
          (:Completed
            (Class|PhysicsConstraintComponent|BreakConstraint (Variables|Default|GetPhysicsConstraint))
            (Class|PhysicsConstraintComponent|BreakConstraint (Variables|Default|GetPhysicsConstraint1))
            (Variables|Default|Setbroken true)
            (Class|PrimitiveComponent|SetAngularDamping (Variables|Default|GetHalfGateLeft) 0.0)
            (Class|PrimitiveComponent|SetAngularDamping (Variables|Default|GetHalfGateRight) 0.0)))))))

(event EventBeginPlay
  (Utilities|FlowControl|Delay 0.2)
  (Variables|Default|Setready true))

(fn ConstructionScript)