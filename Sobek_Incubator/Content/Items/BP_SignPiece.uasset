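; BP_SignPiece is a puzzle item that the player picks up from and places onto sign spots.
; On Interact, a connected piece targeted by the player attaches to the hand socket and re-enables its spot's collision.
; A held piece snaps to the targeted Sign-tagged BP_SignSpot and disables that spot's collision.
; Placement sets RightSpot by comparing the spot with its Reference, then calls CallWrongCode on the player either way.
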(event EventBeginPlay
  (bind _asthird_person_character (Utilities|Casting|CastToThirdPersonCharacter (Game|Player|GetPlayerPawn 0)))
  (Input|EnableInput (Game|GetPlayerController 0))
  (Variables|Default|Setplayer _asthird_person_character))

(event Input|ActionEvents|InputActionInteract
  (params (Key :type Key%20Structure :default "None"))
  (bind _self self)
  (:Pressed
    (bind _asthird_person_character (Utilities|Casting|CastToThirdPersonCharacter (Game|Player|GetPlayerPawn 0)))
    (if (Variables|Default|GetConnected)
      (if (and (== (Utilities|GetClass (Variables|/Game/_StarterContent/ThirdPersonBP/Blueprints/ThirdPersonCharacter.ThirdPersonCharacter_C|GetcurrentItem _asthird_person_character)) 0) (== (Variables|/Game/_StarterContent/ThirdPersonBP/Blueprints/ThirdPersonCharacter.ThirdPersonCharacter_C|GethitActor _asthird_person_character) _self))
        (Collision|SetActorEnableCollision (Variables|Default|GetTriggerBox) true)
        (Transformation|AttachComponentToComponent (Variables|/Script/Engine.Character|GetMesh _asthird_person_character) "RightHandItem" "SnapToTarget" "SnapToTarget" "KeepWorld" true)
        (Audio|PlaySound2D "/Game/Sound/Pickup_Cue.Pickup_Cue" 1.0 1.0 0.0 0 0)
        (Variables|/Game/_StarterContent/ThirdPersonBP/Blueprints/ThirdPersonCharacter.ThirdPersonCharacter_C|SetcurrentItem _asthird_person_character self)
        (Physics|SetEnableGravity (Variables|Debug|GetStaticMeshComponent) true)
        (Variables|Default|SetConnected false)
        (Variables|/Game/_StarterContent/ThirdPersonBP/Blueprints/ThirdPersonCharacter.ThirdPersonCharacter_C|SetisAttached _asthird_person_character true)
        (Variables|Default|SetRightSpot false))
      (else
        (bind _asbp_sign_spot (Utilities|Casting|CastToBP_SignSpot (Variables|/Game/_StarterContent/ThirdPersonBP/Blueprints/ThirdPersonCharacter.ThirdPersonCharacter_C|GethitActor _asthird_person_character)))
        (if (and (Actor|ActorHasTag (Variables|/Game/_StarterContent/ThirdPersonBP/Blueprints/ThirdPersonCharacter.ThirdPersonCharacter_C|GethitActor _asthird_person_character) "Sign") (== (Variables|/Game/_StarterContent/ThirdPersonBP/Blueprints/ThirdPersonCharacter.ThirdPersonCharacter_C|GetcurrentItem _asthird_person_character) _self))
          (bind _output_get (Variables|Default|SetTriggerBox _asbp_sign_spot))
          (Collision|SetActorEnableCollision _output_get false)
          (Transformation|DetachFromActor "KeepWorld" "KeepWorld" "KeepWorld")
          (Collision|SetCollisionEnabled (Variables|Debug|GetStaticMeshComponent) "QueryOnly")
          (Physics|SetEnableGravity (Variables|Debug|GetStaticMeshComponent) false)
          (Transformation|SetActorLocationAndRotation (.location (Transformation|GetActorTransform _output_get)) (.rotation (Transformation|GetActorTransform _output_get)))
          (Variables|Default|SetConnected true)
          (Variables|/Game/_StarterContent/ThirdPersonBP/Blueprints/ThirdPersonCharacter.ThirdPersonCharacter_C|SetcurrentItem _asthird_person_character 0)
          (Variables|/Game/_StarterContent/ThirdPersonBP/Blueprints/ThirdPersonCharacter.ThirdPersonCharacter_C|SetisAttached _asthird_person_character false)
          (Variables|/Game/_StarterContent/ThirdPersonBP/Blueprints/ThirdPersonCharacter.ThirdPersonCharacter_C|SetItem%20Pickup _asthird_person_character false)
          (Audio|PlaySound2D "/Game/Sound/Place_Cue.Place_Cue" 0.5 3.0 0.0 0 0)
          (if (== _output_get (Variables|Default|GetReference))
            (Variables|Default|SetRightSpot true)
            (else
              (Variables|Default|SetRightSpot false)))
          (Default|CallWrongCode (Variables|Default|Getplayer)))))))

(fn ConstructionScript)