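; Power generator that accepts a carried extension cable and, once powered, readies the subway train to finish the level.
; Inside the box trigger, Interact snaps a connector, identified by display name, onto a dummy point and sets Check1; an unfinished branch handles unplugging.
; Tick waits for Check1 and Check2 (not set here), then once plays a power-up sound, turns the light green, sets TrainReady and destroys the car door.
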(event OnComponentEndOverlap(Box)
  (params (OverlappedComponent :type Primitive%20Component%20Object%20Reference) (OtherActor :type Actor%20Object%20Reference) (OtherComp :type Primitive%20Component%20Object%20Reference) (OtherBodyIndex :type Integer))
  (bind _asthird_person_character (Utilities|Casting|CastToThirdPersonCharacter OtherActor))
  (Variables|/Game/_StarterContent/ThirdPersonBP/Blueprints/ThirdPersonCharacter.ThirdPersonCharacter_C|SetuiText _asthird_person_character "")
  (Variables|Default|SetSetIn false))

(event OnComponentBeginOverlap(Box)
  (params (OverlappedComponent :type Primitive%20Component%20Object%20Reference) (OtherActor :type Actor%20Object%20Reference) (OtherComp :type Primitive%20Component%20Object%20Reference) (OtherBodyIndex :type Integer) (bFromSweep :type Boolean) (SweepResult :type Hit%20Result%20Structure%20%28by%20ref%29))
  (bind _asthird_person_character (Utilities|Casting|CastToThirdPersonCharacter OtherActor))
  (Utilities|IsValid (Variables|/Game/_StarterContent/ThirdPersonBP/Blueprints/ThirdPersonCharacter.ThirdPersonCharacter_C|GetcurrentItem _asthird_person_character)
    (:Is%20Valid
      (if (or (Utilities|Enum|Equal(Enum) (Utilities|GetDisplayName (Variables|/Game/_StarterContent/ThirdPersonBP/Blueprints/ThirdPersonCharacter.ThirdPersonCharacter_C|GetcurrentItem _asthird_person_character)) "ExtensionConnector") (Utilities|Enum|Equal(Enum) (Utilities|GetDisplayName (Variables|/Game/_StarterContent/ThirdPersonBP/Blueprints/ThirdPersonCharacter.ThirdPersonCharacter_C|GetcurrentItem _asthird_person_character)) "ExtensionConnectorEnd"))
        (Variables|/Game/_StarterContent/ThirdPersonBP/Blueprints/ThirdPersonCharacter.ThirdPersonCharacter_C|SetuiText _asthird_person_character "Press E to attach power cable"))
      (Variables|Default|SetSetIn true))))

(event EventTick
  (params (DeltaSeconds :type Float%20%28single-precision%29))
  (if (and (Variables|Default|GetCheck1) (Variables|Default|GetCheck2))
    (Utilities|FlowControl|DoOnce false
      (:Completed
        (Audio|PlaySoundatLocation "/Game/Sound/PoweringUp_Cue.PoweringUp_Cue" (Transformation|GetWorldLocation (Variables|Default|GetStaticMesh)) "0, 0, 0" 1.0 1.0 0.0 0 0 0)
        (Rendering|Components|Light|SetLightColor (Variables|Default|GetPointLight) "(R=0.000000,G=1.000000,B=0.001896,A=1.000000)" true)
        (Variables|Default|SetTrainReady true)
        (Development|PrintString "Level Finish Ready")
        (Actor|DestroyActor (Variables|Default|GetSubwayCarDoor))))))

(event Input|ActionEvents|InputActionInteract
  (params (Key :type Key%20Structure :default "None"))
  (bind _player (Variables|Default|GetPlayer))
  (:Pressed
    (Utilities|IsValid (Variables|/Game/_StarterContent/ThirdPersonBP/Blueprints/ThirdPersonCharacter.ThirdPersonCharacter_C|GetcurrentItem (stale OnComponentBeginOverlap(Box) _asthird_person_character))
      (:Is%20Valid
        (if (or (Utilities|Enum|Equal(Enum) (Utilities|GetDisplayName (Variables|/Game/_StarterContent/ThirdPersonBP/Blueprints/ThirdPersonCharacter.ThirdPersonCharacter_C|GetcurrentItem (stale OnComponentBeginOverlap(Box) _asthird_person_character))) "ExtensionConnector") (Utilities|Enum|Equal(Enum) (Utilities|GetDisplayName (Variables|/Game/_StarterContent/ThirdPersonBP/Blueprints/ThirdPersonCharacter.ThirdPersonCharacter_C|GetcurrentItem (stale OnComponentBeginOverlap(Box) _asthird_person_character))) "ExtensionConnectorEnd"))
          (if (Variables|Default|GetSetIn)
            (if (Variables|Default|GetConnected)
              ;[1 1 1] fix this
              (if (Utilities|Enum|Equal(Enum) (Utilities|GetDisplayName (Variables|/Game/_StarterContent/ThirdPersonBP/Blueprints/ThirdPersonCharacter.ThirdPersonCharacter_C|GethitActor (Variables|Default|GetPlayer))) (Utilities|GetDisplayName (stale _output_get))) :!label _label
                (Variables|Default|SetConnected false)
                (Variables|Default|SetCheck1 false))
              (else
                (bind _output_get (Variables|Default|SetExtensionConnector (Variables|/Game/_StarterContent/ThirdPersonBP/Blueprints/ThirdPersonCharacter.ThirdPersonCharacter_C|GetcurrentItem (stale OnComponentBeginOverlap(Box) _asthird_person_character))))
                (Transformation|AttachComponentToComponent (Variables|Default|GetExtensionConnector) (Variables|Default|GetDummy) "None" "SnapToTarget" "KeepWorld" "KeepWorld" true)
                (Collision|SetCollisionEnabled (Actor|GetComponentbyClass (Variables|Default|GetExtensionConnector) "/Script/Engine.StaticMeshComponent") "QueryOnly")
                (Variables|/Game/_StarterContent/ThirdPersonBP/Blueprints/ThirdPersonCharacter.ThirdPersonCharacter_C|SetcurrentItem (stale OnComponentBeginOverlap(Box) _asthird_person_character) 0)
                (Variables|Default|SetConnected true)
                (Variables|/Game/_StarterContent/ThirdPersonBP/Blueprints/ThirdPersonCharacter.ThirdPersonCharacter_C|SetisAttached _player false)
                (Variables|/Game/_StarterContent/ThirdPersonBP/Blueprints/ThirdPersonCharacter.ThirdPersonCharacter_C|SetItem%20Pickup _player false)
                (Variables|/Game/_StarterContent/ThirdPersonBP/Blueprints/ThirdPersonCharacter.ThirdPersonCharacter_C|SetIdling _player true)
                (Audio|PlaySound2D "/Game/Sound/GarageClick_Cue.GarageClick_Cue" 0.3 15.0 0.0 0 0)
                (if (not (Variables|Default|GetActive))
                  (Variables|Default|SetCheck1 true)))))
          (else
            (goto _label)))))))

(fn ConstructionScript)