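; BP_Map is an item actor whose static mesh returns to its starting placement when the player resets from the pause menu.
; Shortly after BeginPlay it stores the mesh's world transform and binds Reset to the reset dispatcher on the ThirdPersonCharacter's PauseMenu.
; Reset zeroes the mesh's physics linear velocity and restores the saved transform without sweep or teleport.
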(event Custom|Reset
  (Physics|SetPhysicsLinearVelocity (Variables|Default|GetStaticMesh) "0, 0, 0" false "None")
  (Transformation|SetWorldTransform (Variables|Default|GetStaticMesh) (Variables|Default|GetLocation) false false))

(event Collision|EventActorBeginOverlap
  (params (OtherActor :type Actor%20Object%20Reference)))

(event EventTick
  (params (DeltaSeconds :type Float%20%28single-precision%29)))

(event EventBeginPlay
  (Utilities|FlowControl|Delay 0.2)
  (Variables|Default|SetLocation (Transformation|GetWorldTransform (Variables|Default|GetStaticMesh)))
  (bind _asthird_person_character (Utilities|Casting|CastToThirdPersonCharacter (Game|Player|GetPlayerPawn 0)))
  (EventDispatchers|BindEventtoResetDispatch (Variables|/Game/_StarterContent/ThirdPersonBP/Blueprints/ThirdPersonCharacter.ThirdPersonCharacter_C|GetPauseMenu _asthird_person_character) (delegate Custom|Reset)))

(fn ConstructionScript)