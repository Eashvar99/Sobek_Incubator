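; BP_BoothDoor is an interactable booth door that the player opens with E while overlapping its OpenableSide trigger.
; The trigger toggles input and the character's InDoor flag, and interaction requires the character to be empty-handed with a "Door"-tagged hit actor.
; A locked door plays a sound and rattle timeline, otherwise it swings open via timeline, nudging the player with alternating movement input and removing its tag.
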(event OnComponentBeginOverlap(OpenableSide)
  (params (OverlappedComponent :type Primitive%20Component%20Object%20Reference) (OtherActor :type Actor%20Object%20Reference) (OtherComp :type Primitive%20Component%20Object%20Reference) (OtherBodyIndex :type Integer) (bFromSweep :type Boolean) (SweepResult :type Hit%20Result%20Structure%20%28by%20ref%29))
  (Input|EnableInput (Game|GetPlayerController 0))
  (bind _asthird_person_character (Utilities|Casting|CastToThirdPersonCharacter OtherActor))
  (Variables|/Game/_StarterContent/ThirdPersonBP/Blueprints/ThirdPersonCharacter.ThirdPersonCharacter_C|SetInDoor _asthird_person_character true))

(event OnComponentEndOverlap(OpenableSide)
  (params (OverlappedComponent :type Primitive%20Component%20Object%20Reference) (OtherActor :type Actor%20Object%20Reference) (OtherComp :type Primitive%20Component%20Object%20Reference) (OtherBodyIndex :type Integer))
  (Input|DisableInput (Game|GetPlayerController 0))
  (bind _asthird_person_character (Utilities|Casting|CastToThirdPersonCharacter OtherActor))
  (Variables|/Game/_StarterContent/ThirdPersonBP/Blueprints/ThirdPersonCharacter.ThirdPersonCharacter_C|SetInDoor _asthird_person_character false))

(event Input|KeyboardEvents|E
  (params (Key :type Key%20Structure :default "None"))
  (:Pressed
    (bind _asthird_person_character (Utilities|Casting|CastToThirdPersonCharacter (stale OnComponentBeginOverlap(OpenableSide) OtherActor)))
    (if (not (Variables|/Game/_StarterContent/ThirdPersonBP/Blueprints/ThirdPersonCharacter.ThirdPersonCharacter_C|GetisGrabbed _asthird_person_character))
      (Utilities|IsValid (Variables|/Game/_StarterContent/ThirdPersonBP/Blueprints/ThirdPersonCharacter.ThirdPersonCharacter_C|GethitActor _asthird_person_character)
        (:Is%20Valid
          (if (Actor|ActorHasTag (Variables|/Game/_StarterContent/ThirdPersonBP/Blueprints/ThirdPersonCharacter.ThirdPersonCharacter_C|GethitActor _asthird_person_character) "Door")
            (if (Variables|Default|GetDoor_Closed)
              (if (Variables|Default|GetLockedside)
                (Utilities|FlowControl|DoOnce false :!label _label
                  (:Completed
                    (Audio|PlaySoundatLocation "/Game/Sound/Locked_Cue.Locked_Cue" (Transformation|GetWorldLocation) "0, 0, 0" 1.0 1.0 0.0 0 0 0)
                    (bind _locked (Timeline|Locked PlayFromStart)
                      (:Update
                        (Transformation|SetRelativeRotation (Math|Rotator|MakeRotator 0.0 0.0 _locked) false false))
                      (:Finished
                        (Variables|Default|SetLockCheck true)
                        (goto _label Reset)))))
                (else
                  (Variables|Default|SetDoor_Closed false)
                  (Audio|PlaySoundatLocation (Variables|Default|GetSound) (Transformation|GetWorldLocation) "0, 0, 0" 1.0 1.0 0.0 0 0 0)
                  (bind _open_close (Timeline|Open/Close Play)
                    (:Update
                      (Transformation|SetRelativeRotation (Math|Rotator|MakeRotator 0.0 0.0 _open_close) false false)
                      (bind _asthird_person_character_2 (Utilities|Casting|CastToThirdPersonCharacter (Game|Player|GetPlayerPawn 0)))
                      (bind _isa (Utilities|FlowControl|FlipFlop)
                        (:A
                          _)
                        (:B
                          _))
                      (Pawn|Input|AddMovementInput _asthird_person_character_2 "1.000000,0.000000, 0" (Math|Float|SelectFloat 0.01 -0.01 _isa) false)
                      (Utilities|Array|RemoveItem (Variables|Actor|GetTags) "Door"))))))))))))

(fn ConstructionScript)