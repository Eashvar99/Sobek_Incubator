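; House door actor that acts locked when used and triggers the HouseTransition2 level sequence.
; Trigger volumes on both sides toggle door input and the character's InDoor flag.
; Pressing E on the hit Door-tagged actor plays a locked sound and timeline rotation, starting the sequence through a DoOnce.
; The unlock-and-open logic is disconnected, and the locked-side check has no effect.
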(event OnComponentBeginOverlap(OpenableSide)
  (params (OverlappedComponent :type Primitive%20Component%20Object%20Reference) (OtherActor :type Actor%20Object%20Reference) (OtherComp :type Primitive%20Component%20Object%20Reference) (OtherBodyIndex :type Integer) (bFromSweep :type Boolean) (SweepResult :type Hit%20Result%20Structure%20%28by%20ref%29))
  (Input|EnableInput (Game|GetPlayerController 0))
  (bind _asthird_person_character (Utilities|Casting|CastToThirdPersonCharacter OtherActor))
  (Variables|/Game/_StarterContent/ThirdPersonBP/Blueprints/ThirdPersonCharacter.ThirdPersonCharacter_C|SetInDoor _asthird_person_character true))

(event OnComponentEndOverlap(OpenableSide)
  (params (OverlappedComponent :type Primitive%20Component%20Object%20Reference) (OtherActor :type Actor%20Object%20Reference) (OtherComp :type Primitive%20Component%20Object%20Reference) (OtherBodyIndex :type Integer))
  (Input|DisableInput (Game|GetPlayerController 0))
  (bind _asthird_person_character (Utilities|Casting|CastToThirdPersonCharacter OtherActor))
  (Variables|/Game/_StarterContent/ThirdPersonBP/Blueprints/ThirdPersonCharacter.ThirdPersonCharacter_C|SetInDoor _asthird_person_character false))

(event OnComponentBeginOverlap(Closedside)
  (params (OverlappedComponent :type Primitive%20Component%20Object%20Reference) (OtherActor :type Actor%20Object%20Reference) (OtherComp :type Primitive%20Component%20Object%20Reference) (OtherBodyIndex :type Integer) (bFromSweep :type Boolean) (SweepResult :type Hit%20Result%20Structure%20%28by%20ref%29))
  (bind _asthird_person_character (Utilities|Casting|CastToThirdPersonCharacter OtherActor))
  (Variables|/Game/_StarterContent/ThirdPersonBP/Blueprints/ThirdPersonCharacter.ThirdPersonCharacter_C|SetInDoor _asthird_person_character true)
  (Variables|Default|SetLockedside true)
  (Input|EnableInput (Game|GetPlayerController 0))
  (bind _asthird_person_character_2 (Utilities|Casting|CastToThirdPersonCharacter (stale OnComponentBeginOverlap(OpenableSide) OtherActor)))
  (Variables|/Game/_StarterContent/ThirdPersonBP/Blueprints/ThirdPersonCharacter.ThirdPersonCharacter_C|SetInDoor _asthird_person_character_2 true))

(event OnComponentEndOverlap(Closedside)
  (params (OverlappedComponent :type Primitive%20Component%20Object%20Reference) (OtherActor :type Actor%20Object%20Reference) (OtherComp :type Primitive%20Component%20Object%20Reference) (OtherBodyIndex :type Integer))
  (bind _asthird_person_character (Utilities|Casting|CastToThirdPersonCharacter OtherActor))
  (Variables|/Game/_StarterContent/ThirdPersonBP/Blueprints/ThirdPersonCharacter.ThirdPersonCharacter_C|SetInDoor _asthird_person_character false)
  (Variables|Default|SetLockedside false)
  (Input|DisableInput (Game|GetPlayerController 0))
  (bind _asthird_person_character_2 (Utilities|Casting|CastToThirdPersonCharacter (stale OnComponentEndOverlap(OpenableSide) OtherActor)))
  (Variables|/Game/_StarterContent/ThirdPersonBP/Blueprints/ThirdPersonCharacter.ThirdPersonCharacter_C|SetInDoor _asthird_person_character_2 false))

(event OnComponentBeginOverlap(Check)
  (params (OverlappedComponent :type Primitive%20Component%20Object%20Reference) (OtherActor :type Actor%20Object%20Reference) (OtherComp :type Primitive%20Component%20Object%20Reference) (OtherBodyIndex :type Integer) (bFromSweep :type Boolean) (SweepResult :type Hit%20Result%20Structure%20%28by%20ref%29)))

(event EventBeginPlay
  (bind _outactor (Sequencer|Player|CreateLevelSequencePlayer "/Game/Cinematics/HouseLevel/HouseTransition2.HouseTransition2"))
  (Variables|Default|SetTrans _outactor))

(event Input|KeyboardEvents|E
  (params (Key :type Key%20Structure :default "None"))
  (:Pressed
    (bind _asthird_person_character (Utilities|Casting|CastToThirdPersonCharacter (stale OnComponentBeginOverlap(Check) OtherActor)))
    (if (not (Variables|/Game/_StarterContent/ThirdPersonBP/Blueprints/ThirdPersonCharacter.ThirdPersonCharacter_C|GetisGrabbed _asthird_person_character))
      (Utilities|IsValid (Variables|/Game/_StarterContent/ThirdPersonBP/Blueprints/ThirdPersonCharacter.ThirdPersonCharacter_C|GethitActor _asthird_person_character)
        (:Is%20Valid
          (if (Actor|ActorHasTag (Variables|/Game/_StarterContent/ThirdPersonBP/Blueprints/ThirdPersonCharacter.ThirdPersonCharacter_C|GethitActor _asthird_person_character) "Door")
            (if (Variables|Default|GetDoor_Closed)
              (if (Variables|Default|GetLockedside)
                _
                (else
                  _))
              (Utilities|FlowControl|DoOnce false :!label _label
                (:Completed
                  (Audio|PlaySoundatLocation "/Game/Sound/Locked_Cue.Locked_Cue" (Transformation|GetWorldLocation (Variables|Default|GetDoor)) "0, 0, 0" 1.0 1.0 0.0 0 0 0)
                  (bind _locked (Timeline|Locked PlayFromStart)
                    (:Update
                      (Transformation|SetRelativeRotation (Variables|Default|GetDoor) (Math|Rotator|MakeRotator 0.0 0.0 _locked) false false)
                      (Utilities|FlowControl|DoOnce false
                        (:Completed
                          (Sequencer|Player|Play (Variables|/Script/LevelSequence.LevelSequenceActor|GetSequencePlayer (Variables|Default|GetTrans)) :!class /Script/MovieScene.MovieSceneSequencePlayer))))
                    (:Finished
                      (Variables|Default|SetLockCheck true)
                      (goto _label Reset))))))))))))

(fn ConstructionScript)