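; BP_Ladder is a climbable ladder that flags the ThirdPersonCharacter as able to climb and handles dismounting and mounting at both ends.
; Overlap volumes set the character's ladder state and restore walking and camera yaw limits on exit.
; Reaching the top while climbing plays a timeline that lifts the character forward over the edge.
; Interact at the top plays a descent timeline blending transform and camera onto the ladder, with level-dependent footstep sounds.
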(event OnComponentBeginOverlap(ClimbVolume)
  (params (OverlappedComponent :type Primitive%20Component%20Object%20Reference) (OtherActor :type Actor%20Object%20Reference) (OtherComp :type Primitive%20Component%20Object%20Reference) (OtherBodyIndex :type Integer) (bFromSweep :type Boolean) (SweepResult :type Hit%20Result%20Structure%20%28by%20ref%29))
  (bind _asthird_person_character (Utilities|Casting|CastToThirdPersonCharacter OtherActor))
  (Variables|/Game/_StarterContent/ThirdPersonBP/Blueprints/ThirdPersonCharacter.ThirdPersonCharacter_C|SetcanClimbLadder _asthird_person_character true)
  (Variables|/Game/_StarterContent/ThirdPersonBP/Blueprints/ThirdPersonCharacter.ThirdPersonCharacter_C|SetCurrentLadder _asthird_person_character self))

(event OnComponentEndOverlap(ClimbVolume)
  (params (OverlappedComponent :type Primitive%20Component%20Object%20Reference) (OtherActor :type Actor%20Object%20Reference) (OtherComp :type Primitive%20Component%20Object%20Reference) (OtherBodyIndex :type Integer))
  (bind _returnvalue (Game|GetPlayerCameraManager 0))
  (bind _asthird_person_character (Utilities|Casting|CastToThirdPersonCharacter OtherActor))
  (Pawn|Components|CharacterMovement|SetMovementMode (Variables|/Script/Engine.Character|GetCharacterMovement _asthird_person_character) "MOVE_Walking" 0)
  (Variables|/Script/Engine.PlayerCameraManager|SetViewYawMax _returnvalue 359.998993)
  (Variables|/Script/Engine.PlayerCameraManager|SetViewYawMin _returnvalue 0.0))

(event OnComponentBeginOverlap(BotDisembark)
  (params (OverlappedComponent :type Primitive%20Component%20Object%20Reference) (OtherActor :type Actor%20Object%20Reference) (OtherComp :type Primitive%20Component%20Object%20Reference) (OtherBodyIndex :type Integer) (bFromSweep :type Boolean) (SweepResult :type Hit%20Result%20Structure%20%28by%20ref%29))
  (bind _returnvalue (Game|GetPlayerCameraManager 0))
  (bind _asthird_person_character (Utilities|Casting|CastToThirdPersonCharacter OtherActor))
  (if (Variables|/Game/_StarterContent/ThirdPersonBP/Blueprints/ThirdPersonCharacter.ThirdPersonCharacter_C|GetisClimbing _asthird_person_character)
    (Variables|/Game/_StarterContent/ThirdPersonBP/Blueprints/ThirdPersonCharacter.ThirdPersonCharacter_C|SetcanClimbLadder _asthird_person_character false)
    (Variables|/Game/_StarterContent/ThirdPersonBP/Blueprints/ThirdPersonCharacter.ThirdPersonCharacter_C|SetisClimbing _asthird_person_character false)
    (Pawn|Components|CharacterMovement|SetMovementMode (Variables|/Script/Engine.Character|GetCharacterMovement _asthird_person_character) "MOVE_Walking" 0)
    (Variables|/Script/Engine.PlayerCameraManager|SetViewYawMax _returnvalue 359.998993)
    (Variables|/Script/Engine.PlayerCameraManager|SetViewYawMin _returnvalue 0.0)
    (Variables|/Game/_StarterContent/ThirdPersonBP/Blueprints/ThirdPersonCharacter.ThirdPersonCharacter_C|SetBotLadder _asthird_person_character true)
    (else
      (Variables|/Game/_StarterContent/ThirdPersonBP/Blueprints/ThirdPersonCharacter.ThirdPersonCharacter_C|SetBotLadder _asthird_person_character true))))

(event OnComponentBeginOverlap(TopDisembark)
  (params (OverlappedComponent :type Primitive%20Component%20Object%20Reference) (OtherActor :type Actor%20Object%20Reference) (OtherComp :type Primitive%20Component%20Object%20Reference) (OtherBodyIndex :type Integer) (bFromSweep :type Boolean) (SweepResult :type Hit%20Result%20Structure%20%28by%20ref%29))
  (bind _returnvalue (Game|GetPlayerCameraManager 0))
  (if (not (Variables|Default|GetDisembark))
    (bind _asthird_person_character (Utilities|Casting|CastToThirdPersonCharacter OtherActor))
    (Input|EnableInput (Game|GetPlayerController 0))
    (if (Variables|/Game/_StarterContent/ThirdPersonBP/Blueprints/ThirdPersonCharacter.ThirdPersonCharacter_C|GetisClimbing _asthird_person_character)
      (Pawn|Components|CharacterMovement|SetMovementMode (Variables|/Script/Engine.Character|GetCharacterMovement _asthird_person_character) "MOVE_Walking" 0)
      (Variables|/Script/Engine.PlayerCameraManager|SetViewYawMax _returnvalue 359.998993)
      (Variables|/Script/Engine.PlayerCameraManager|SetViewYawMin _returnvalue 0.0)
      (Utilities|FlowControl|DoOnce false :!label _label
        (:Completed
          (bind _asthird_person_character_2 (Utilities|Casting|CastToThirdPersonCharacter (Game|Player|GetPlayerPawn 0)))
          (Variables|/Game/_StarterContent/ThirdPersonBP/Blueprints/ThirdPersonCharacter.ThirdPersonCharacter_C|SetTopLadder _asthird_person_character_2 true)
          (Input|DisableInput _asthird_person_character_2 (Game|GetPlayerController 0))
          (Pawn|Components|CharacterMovement|SetMovementMode (Variables|/Script/Engine.Character|GetCharacterMovement _asthird_person_character_2) "MOVE_Flying" 0)
          (Variables|Default|SetBeforeClimb (Transformation|GetActorTransform _asthird_person_character_2))
          (bind (_direction _rotate _climbtransformup _climbforward) (Timeline|Climb PlayFromStart)
            (:Update
              (Transformation|SetActorRelativeLocation _asthird_person_character_2 (Math|Vector|MakeVector (+ (.x (.location (Variables|Default|GetBeforeClimb))) (* (.x (Math|Vector|GetForwardVector (.rotation (Variables|Default|GetBeforeClimb)))) _climbforward)) (+ (.y (.location (Variables|Default|GetBeforeClimb))) (* (.y (Math|Vector|GetForwardVector (.rotation (Variables|Default|GetBeforeClimb)))) _climbforward)) (+ _climbtransformup (.z (.location (Variables|Default|GetBeforeClimb)))))))
            (:Finished
              (Collision|SetActorEnableCollision _asthird_person_character_2 true)
              (Input|EnableInput _asthird_person_character_2 (Game|GetPlayerController 0))
              (Pawn|Components|CharacterMovement|SetMovementMode (Variables|/Script/Engine.Character|GetCharacterMovement _asthird_person_character_2) "MOVE_Walking" 0)
              (Variables|/Game/_StarterContent/ThirdPersonBP/Blueprints/ThirdPersonCharacter.ThirdPersonCharacter_C|SetcanClimbLadder _asthird_person_character_2 false)
              (Variables|/Game/_StarterContent/ThirdPersonBP/Blueprints/ThirdPersonCharacter.ThirdPersonCharacter_C|SetisClimbing _asthird_person_character_2 false)
              (Variables|/Game/_StarterContent/ThirdPersonBP/Blueprints/ThirdPersonCharacter.ThirdPersonCharacter_C|SetTopLadder _asthird_person_character_2 false)
              (goto _label Reset)))))
      (else
        (Variables|/Game/_StarterContent/ThirdPersonBP/Blueprints/ThirdPersonCharacter.ThirdPersonCharacter_C|SetTopLadder _asthird_person_character true)))))

(event OnComponentEndOverlap(TopDisembark)
  (params (OverlappedComponent :type Primitive%20Component%20Object%20Reference) (OtherActor :type Actor%20Object%20Reference) (OtherComp :type Primitive%20Component%20Object%20Reference) (OtherBodyIndex :type Integer))
  (bind _asthird_person_character (Utilities|Casting|CastToThirdPersonCharacter OtherActor))
  (Input|DisableInput (Game|GetPlayerController 0))
  (Variables|/Game/_StarterContent/ThirdPersonBP/Blueprints/ThirdPersonCharacter.ThirdPersonCharacter_C|SetTopLadder _asthird_person_character false))

(event OnComponentEndOverlap(BotDisembark)
  (params (OverlappedComponent :type Primitive%20Component%20Object%20Reference) (OtherActor :type Actor%20Object%20Reference) (OtherComp :type Primitive%20Component%20Object%20Reference) (OtherBodyIndex :type Integer))
  (bind _asthird_person_character (Utilities|Casting|CastToThirdPersonCharacter OtherActor))
  (Variables|/Game/_StarterContent/ThirdPersonBP/Blueprints/ThirdPersonCharacter.ThirdPersonCharacter_C|SetBotLadder _asthird_person_character false))

(event EventBeginPlay)

(event Input|ActionEvents|InputActionInteract
  (params (Key :type Key%20Structure :default "None"))
  (:Pressed
    (bind _asthird_person_character (Utilities|Casting|CastToThirdPersonCharacter (Game|Player|GetPlayerPawn 0)))
    (if (and (== (Utilities|GetClass (Variables|/Game/_StarterContent/ThirdPersonBP/Blueprints/ThirdPersonCharacter.ThirdPersonCharacter_C|GethitActor _asthird_person_character)) "BP_Ladder_C") (Variables|/Game/_StarterContent/ThirdPersonBP/Blueprints/ThirdPersonCharacter.ThirdPersonCharacter_C|GetTopLadder _asthird_person_character))
      (Variables|Default|SetDisembark true)
      (Variables|/Game/_StarterContent/ThirdPersonBP/Blueprints/ThirdPersonCharacter.ThirdPersonCharacter_C|SetTopLadder _asthird_person_character false)
      (Input|DisableInput _asthird_person_character (Game|GetPlayerController 0))
      (Pawn|Components|CharacterMovement|SetMovementMode (Variables|/Script/Engine.Character|GetCharacterMovement _asthird_person_character) "MOVE_Flying" 0)
      (Variables|/Script/Engine.CameraComponent|SetbUsePawnControlRotation (Variables|/Game/_StarterContent/ThirdPersonBP/Blueprints/ThirdPersonCharacter.ThirdPersonCharacter_C|GetFollowCamera _asthird_person_character) false)
      (Variables|Default|SetCameraRotate (Transformation|GetWorldRotation (Variables|/Game/_StarterContent/ThirdPersonBP/Blueprints/ThirdPersonCharacter.ThirdPersonCharacter_C|GetFollowCamera _asthird_person_character)))
      (bind _output_get (Variables|Default|SetBeforeDescent (Transformation|GetActorTransform _asthird_person_character)))
      (bind (_direction _newtrack_0 _camerayawyeet) (Timeline|BottomLadder PlayFromStart)
        (:Update
          (Transformation|SetActorTransform _asthird_person_character (Math|Transform|MakeTransform (.location (Math|Transform|Lerp(Transform) _output_get (Transformation|GetWorldTransform (Variables|Default|GetDescentPos)) _newtrack_0)) (.rotation (Math|Transform|Lerp(Transform) _output_get (Transformation|GetWorldTransform (Variables|Default|GetDescentPos)) _newtrack_0)) "1,1,1"))
          (Transformation|SetWorldRotation (Variables|/Game/_StarterContent/ThirdPersonBP/Blueprints/ThirdPersonCharacter.ThirdPersonCharacter_C|GetFollowCamera _asthird_person_character) (Math|Rotator|MakeRotator (.Roll (Math|Rotator|BreakRotator (.Rotation (Math|Transform|BreakTransform (Transformation|GetWorldTransform (Variables|/Script/Engine.Actor|GetRootComponent _asthird_person_character)))))) (.pitch (Math|Rotator|Lerp(Rotator) (Math|Rotator|MakeRotator 0.0 (.pitch (Variables|Default|GetCameraRotate)) 0.0) "0, 0, 0" _camerayawyeet)) (.Yaw (Math|Rotator|BreakRotator (.Rotation (Math|Transform|BreakTransform (Transformation|GetWorldTransform (Variables|/Script/Engine.Actor|GetRootComponent _asthird_person_character))))))) false false))
        (:Finished
          (Variables|/Game/_StarterContent/ThirdPersonBP/Blueprints/ThirdPersonCharacter.ThirdPersonCharacter_C|SetisClimbing _asthird_person_character true)
          (Collision|SetActorEnableCollision _asthird_person_character true)
          (Input|EnableInput _asthird_person_character (Game|GetPlayerController 0))
          (Pawn|Components|CharacterMovement|SetMovementMode (Variables|/Script/Engine.Character|GetCharacterMovement _asthird_person_character) "MOVE_Walking" 0)
          (Pawn|SetControlRotation (Game|GetPlayerController 0) (Transformation|GetWorldRotation (Variables|Default|GetDescentPos)))
          (Variables|/Script/Engine.CameraComponent|SetbUsePawnControlRotation (Variables|/Game/_StarterContent/ThirdPersonBP/Blueprints/ThirdPersonCharacter.ThirdPersonCharacter_C|GetFollowCamera _asthird_person_character) true)
          (Variables|Default|SetDisembark false))
        (:Footsteppy%20sound
          (bind _returnvalue (Game|GetCurrentLevelName true))
          (if (Utilities|Enum|Equal(Enum) _returnvalue "CityLevel_2")
            (Audio|PlaySound2D "/Game/Sound/Footsteps/Footstep_Metal_01_Cue.Footstep_Metal_01_Cue" 1.0 1.0 0.0 0 0)
            (else
              (Audio|PlaySound2D "/Game/Sound/Footsteps/Footstep_Wood_01_Cue.Footstep_Wood_01_Cue" 1.0 1.0 0.0 0 0))))))))

(fn ConstructionScript)