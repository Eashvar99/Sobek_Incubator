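; BP_Key is a collectible key item that the player character can grab.
; Overlap events on its components toggle the actor's input for the first player controller.
; Each Tick polls CanGrabKey on ThirdPersonCharacter, with no overlap check; when set, it adds KeyType to OwnedKeys, destroys the key and clears the flag.
; The construction script selects the key's material from KeyType.
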(event OnComponentBeginOverlap(Overlap)
  (params (OverlappedComponent :type Primitive%20Component%20Object%20Reference) (OtherActor :type Actor%20Object%20Reference) (OtherComp :type Primitive%20Component%20Object%20Reference) (OtherBodyIndex :type Integer) (bFromSweep :type Boolean) (SweepResult :type Hit%20Result%20Structure%20%28by%20ref%29))
  (Input|EnableInput (Game|GetPlayerController 0)))

(event OnComponentEndOverlap(Box)
  (params (OverlappedComponent :type Primitive%20Component%20Object%20Reference) (OtherActor :type Actor%20Object%20Reference) (OtherComp :type Primitive%20Component%20Object%20Reference) (OtherBodyIndex :type Integer))
  (Input|DisableInput (Game|GetPlayerController 0)))

(event EventTick
  (params (DeltaSeconds :type Float%20%28single-precision%29))
  (bind _asthird_person_character (Utilities|Casting|CastToThirdPersonCharacter (Game|Player|GetPlayerPawn 0)))
  (if (Variables|/Game/_StarterContent/ThirdPersonBP/Blueprints/ThirdPersonCharacter.ThirdPersonCharacter_C|GetcanGrabKey _asthird_person_character)
    (Utilities|Array|Add (Variables|/Game/_StarterContent/ThirdPersonBP/Blueprints/ThirdPersonCharacter.ThirdPersonCharacter_C|GetOwnedKeys _asthird_person_character) (Variables|Default|GetKeyType))
    (Actor|DestroyActor)
    (Variables|/Game/_StarterContent/ThirdPersonBP/Blueprints/ThirdPersonCharacter.ThirdPersonCharacter_C|SetcanGrabKey _asthird_person_character false)))

(fn ConstructionScript
  (Rendering|Material|SetMaterial (Variables|Default|GetKey) 0 (Utilities|Select :Index (Variables|Default|GetKeyType) :NewEnumerator0 "/Game/Items/ItemMeshes/M_Key.M_Key" :NewEnumerator1 "/Game/Items/ItemMeshes/M_Test.M_Test")))