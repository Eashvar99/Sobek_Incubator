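; BP_SignSpot is a placement spot that shows its Cube only while the player looks at it holding a sign piece.
; On BeginPlay it caches the player pawn as a ThirdPersonCharacter.
; Each Tick it compares the player's HitActor to itself and checks that CurrentItem is a BP_SignPiece to unhide the Cube.
; It hides the Cube again only when it is no longer the HitActor.
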(event EventBeginPlay
  (bind _asthird_person_character (Utilities|Casting|CastToThirdPersonCharacter (Game|Player|GetPlayerPawn 0)))
  (Variables|Default|SetPlayer _asthird_person_character))

(event EventTick
  (params (DeltaSeconds :type Float%20%28single-precision%29))
  (bind _cube (Variables|Default|GetCube))
  (if (== (Variables|/Game/_StarterContent/ThirdPersonBP/Blueprints/ThirdPersonCharacter.ThirdPersonCharacter_C|GethitActor (Variables|Default|GetPlayer)) self)
    (if (== (Utilities|GetClass (Variables|/Game/_StarterContent/ThirdPersonBP/Blueprints/ThirdPersonCharacter.ThirdPersonCharacter_C|GetcurrentItem (Variables|Default|GetPlayer))) "/Game/Items/BP_SignPiece.BP_SignPiece_C")
      (Development|SetHiddeninGame _cube false false))
    (else
      (Development|SetHiddeninGame _cube true false))))

(fn ConstructionScript)