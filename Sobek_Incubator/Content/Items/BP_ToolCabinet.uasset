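; BP_ToolCabinet is a locked two-door cabinet that the player opens with a key item.
; A box overlap enables and disables input, so E works only in range.
; Pressing E searches the overlapping ThirdPersonCharacter's OwnedKeys for RequiredKeyType and removes each match.
; A match plays a timeline that swings both doors by setting their relative yaw.
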(event OnComponentBeginOverlap(Box)
  (params (OverlappedComponent :type Primitive%20Component%20Object%20Reference) (OtherActor :type Actor%20Object%20Reference) (OtherComp :type Primitive%20Component%20Object%20Reference) (OtherBodyIndex :type Integer) (bFromSweep :type Boolean) (SweepResult :type Hit%20Result%20Structure%20%28by%20ref%29))
  (Input|EnableInput (Game|GetPlayerController 0)))

(event OnComponentEndOverlap(Box)
  (params (OverlappedComponent :type Primitive%20Component%20Object%20Reference) (OtherActor :type Actor%20Object%20Reference) (OtherComp :type Primitive%20Component%20Object%20Reference) (OtherBodyIndex :type Integer))
  (Input|DisableInput (Game|GetPlayerController 0)))

(event Input|KeyboardEvents|E
  (params (Key :type Key%20Structure))
  (:Pressed
    (bind _asthird_person_character (Utilities|Casting|CastToThirdPersonCharacter (stale OnComponentBeginOverlap(Box) OtherActor)))
    (for (_array_element _array_index) (Variables|/Game/_StarterContent/ThirdPersonBP/Blueprints/ThirdPersonCharacter.ThirdPersonCharacter_C|GetOwnedKeys _asthird_person_character)
      (if (Utilities|Enum|Equal(Enum) _array_element (Variables|Default|GetRequiredKeyType))
        (Utilities|Array|RemoveIndex (Variables|/Game/_StarterContent/ThirdPersonBP/Blueprints/ThirdPersonCharacter.ThirdPersonCharacter_C|GetOwnedKeys _asthird_person_character) _array_index)
        (bind (_direction _open_close_left _open_close_right) (Timeline|Timeline_0 Play)
          (:Update
            (Transformation|SetRelativeRotation (Variables|Default|GetLeftDoor) (Math|Rotator|MakeRotator 0.0 0.0 _open_close_left) false false)
            (Transformation|SetRelativeRotation (Variables|Default|GetRightDoor) (Math|Rotator|MakeRotator 0.0 0.0 _open_close_right) false false)))))))

(fn ConstructionScript)