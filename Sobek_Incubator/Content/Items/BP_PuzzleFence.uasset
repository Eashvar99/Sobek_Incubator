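; BP_PuzzleFence is a puzzle fence that the player can fix a held city connector item onto.
; On Interact inside its Box, it moves an Arrow to the player's ray hit, snaps the connector to it and clears the player's held-item state.
; Otherwise, interacting while looking at the attached connector only clears the Connected flag, freeing the fence for another attachment.
; Items are identified by display-name comparisons rather than class or reference.
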(event EventBeginPlay
  (bind _asthird_person_character (Utilities|Casting|CastToThirdPersonCharacter (Game|Player|GetPlayerPawn 0)))
  (Variables|Default|SetPlayer _asthird_person_character)
  (Input|EnableInput (Game|GetPlayerController 0)))

(event EventTick
  (params (DeltaSeconds :type Float%20%28single-precision%29)))

(event Input|ActionEvents|InputActionInteract
  (params (Key :type Key%20Structure :default "None"))
  (bind _player (Variables|Default|GetPlayer))
  (bind _player_2 (Variables|Default|GetPlayer))
  (:Pressed
    (if (Collision|IsOverlappingActor (Variables|Default|GetBox) (Variables|Default|GetPlayer) :!class /Script/Engine.PrimitiveComponent)
      (if (or (Utilities|Enum|Equal(Enum) (Utilities|GetDisplayName (Variables|/Game/_StarterContent/ThirdPersonBP/Blueprints/ThirdPersonCharacter.ThirdPersonCharacter_C|GetcurrentItem _player)) "CityConnector") (Utilities|Enum|Equal(Enum) (Utilities|GetDisplayName (Variables|/Game/_StarterContent/ThirdPersonBP/Blueprints/ThirdPersonCharacter.ThirdPersonCharacter_C|GetcurrentItem _player)) "CityConnectorEnd"))
        (if (not (Variables|Default|GetConnected))
          (bind _output_get (Variables|Default|SetConnector (Variables|/Game/_StarterContent/ThirdPersonBP/Blueprints/ThirdPersonCharacter.ThirdPersonCharacter_C|GetcurrentItem _player)))
          (Transformation|SetWorldLocation (Variables|Default|GetArrow) (Variables|/Game/_StarterContent/ThirdPersonBP/Blueprints/ThirdPersonCharacter.ThirdPersonCharacter_C|GetRayHitLocation _player) false false)
          (Transformation|AttachComponentToComponent _output_get (Variables|Default|GetArrow) "None" "SnapToTarget" "KeepWorld" "KeepWorld" true)
          (Collision|SetCollisionEnabled (Actor|GetComponentbyClass _output_get "/Script/Engine.StaticMeshComponent") "QueryOnly")
          (Variables|Default|SetConnected true)
          (Variables|/Game/_StarterContent/ThirdPersonBP/Blueprints/ThirdPersonCharacter.ThirdPersonCharacter_C|SetItem%20Pickup _player_2 false)
          (Variables|/Game/_StarterContent/ThirdPersonBP/Blueprints/ThirdPersonCharacter.ThirdPersonCharacter_C|SetIdling _player_2 true)
          (Variables|/Game/_StarterContent/ThirdPersonBP/Blueprints/ThirdPersonCharacter.ThirdPersonCharacter_C|SetcurrentItem _player_2 0)
          (Utilities|FlowControl|Delay 0.1)
          (Variables|/Game/_StarterContent/ThirdPersonBP/Blueprints/ThirdPersonCharacter.ThirdPersonCharacter_C|SetisAttached _player_2 false))
        (else
          (if (and (Variables|Default|GetConnected) (Utilities|Enum|Equal(Enum) (Utilities|GetDisplayName (Variables|/Game/_StarterContent/ThirdPersonBP/Blueprints/ThirdPersonCharacter.ThirdPersonCharacter_C|GethitActor _player)) (Utilities|GetDisplayName (Variables|Default|GetConnector)))) :!label _label
            (Variables|Default|SetConnected false))))
      (else
        (goto _label)))))

(fn ConstructionScript)