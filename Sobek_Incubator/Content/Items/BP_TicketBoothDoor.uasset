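; Ticket booth door that stays locked until one of its two destructible glass parts is shattered by a thrown or falling Rock.
; A Rock hit applies heavy damage with a glass-break sound, and the fracture detaches the piece and clears the lock.
; The first Check overlap enables input, so E on the targeted door either plays a locked rattle or swings it open via timelines.
; Opening nudges the player with tiny alternating movement input and removes the Door tag.
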(event OnComponentHit(Destructible)
  (params (HitComponent :type Primitive%20Component%20Object%20Reference) (OtherActor :type Actor%20Object%20Reference) (OtherComp :type Primitive%20Component%20Object%20Reference) (NormalImpulse :type Vector :default "0, 0, 0") (Hit :type Hit%20Result%20Structure%20%28by%20ref%29))
  (bind (_bblockinghit _binitialoverlap _time _distance _location _impactpoint _normal _impactnormal) (Collision|BreakHitResult Hit))
  (Utilities|Casting|CastToRock OtherActor)
  (Physics|SetEnableGravity (Variables|Default|GetDestructible) true)
  (Class|DestructibleComponent|ApplyDamage (Variables|Default|GetDestructible) 1e+03 _impactpoint _impactnormal 1.0)
  (Utilities|FlowControl|DoOnce false
    (:Completed
      (Audio|PlaySoundatLocation "/Game/Sound/GlassBreaking_Cue.GlassBreaking_Cue" _impactpoint "0, 0, 0" 0.8 1.0 0.0 0 0 0))))

(event OnComponentFracture(Destructible)
  (params (HitPoint :type Vector%20%28by%20ref%29 :default "0, 0, 0") (HitDirection :type Vector%20%28by%20ref%29 :default "0, 0, 0"))
  (Variables|Default|SetLockedDoor false)
  (Transformation|DetachFromComponent (Variables|Default|GetDestructible) "KeepWorld" "KeepWorld" "KeepWorld" true))

(event OnComponentBeginOverlap(Check)
  (params (OverlappedComponent :type Primitive%20Component%20Object%20Reference) (OtherActor :type Actor%20Object%20Reference) (OtherComp :type Primitive%20Component%20Object%20Reference) (OtherBodyIndex :type Integer) (bFromSweep :type Boolean) (SweepResult :type Hit%20Result%20Structure%20%28by%20ref%29))
  (Utilities|FlowControl|DoOnce false
    (:Completed
      (Input|EnableInput (Game|GetPlayerController 0)))))

(event OnComponentHit(Destrictible2)
  (params (HitComponent :type Primitive%20Component%20Object%20Reference) (OtherActor :type Actor%20Object%20Reference) (OtherComp :type Primitive%20Component%20Object%20Reference) (NormalImpulse :type Vector :default "0, 0, 0") (Hit :type Hit%20Result%20Structure%20%28by%20ref%29))
  (bind (_bblockinghit _binitialoverlap _time _distance _location _impactpoint _normal _impactnormal) (Collision|BreakHitResult Hit))
  (Utilities|Casting|CastToRock OtherActor)
  (Physics|SetEnableGravity (Variables|Default|GetDestrictible2) true)
  (Class|DestructibleComponent|ApplyDamage (Variables|Default|GetDestrictible2) 1e+03 _impactpoint _impactnormal 1.0)
  (Utilities|FlowControl|DoOnce false
    (:Completed
      (Audio|PlaySoundatLocation "/Game/Sound/GlassBreaking_Cue.GlassBreaking_Cue" _impactpoint "0, 0, 0" 0.8 1.0 0.0 0 0 0))))

(event OnComponentFracture(Destrictible2)
  (params (HitPoint :type Vector%20%28by%20ref%29 :default "0, 0, 0") (HitDirection :type Vector%20%28by%20ref%29 :default "0, 0, 0"))
  (Variables|Default|SetLockedDoor false)
  (Transformation|DetachFromComponent (Variables|Default|GetDestrictible2) "KeepWorld" "KeepWorld" "KeepWorld" true))

(event Input|KeyboardEvents|E
  (params (Key :type Key%20Structure :default "None"))
  (bind _door (Variables|Default|GetDoor))
  (:Pressed
    (bind _asthird_person_character (Utilities|Casting|CastToThirdPersonCharacter (stale OnComponentBeginOverlap(Check) OtherActor)))
    (if (not (Variables|/Game/_StarterContent/ThirdPersonBP/Blueprints/ThirdPersonCharacter.ThirdPersonCharacter_C|GetisGrabbed _asthird_person_character))
      (Utilities|IsValid (Variables|/Game/_StarterContent/ThirdPersonBP/Blueprints/ThirdPersonCharacter.ThirdPersonCharacter_C|GethitActor _asthird_person_character)
        (:Is%20Valid
          (if (Actor|ActorHasTag (Variables|/Game/_StarterContent/ThirdPersonBP/Blueprints/ThirdPersonCharacter.ThirdPersonCharacter_C|GethitActor _asthird_person_character) "Door")
            (if (Variables|Default|GetDoor_Closed)
              (if (Variables|Default|GetLockedDoor)
                (Utilities|FlowControl|DoOnce false :!label _label
                  (:Completed
                    (Audio|PlaySoundatLocation "/Game/Sound/Locked_Cue.Locked_Cue" (Transformation|GetWorldLocation (Variables|Default|GetDoor)) "0, 0, 0" 1.0 1.0 0.0 0 0 0)
                    (bind _locked (Timeline|Locked PlayFromStart)
                      (:Update
                        (Transformation|SetRelativeRotation (Variables|Default|GetDoor) (Math|Rotator|MakeRotator 0.0 0.0 _locked) false false))
                      (:Finished
                        (Variables|Default|SetLockCheck true)
                        (goto _label Reset)))))
                (else
                  (Variables|Default|SetDoor_Closed false)
                  (Audio|PlaySoundatLocation (Variables|Default|GetSound) (Transformation|GetWorldLocation _door) "0, 0, 0" 1.0 1.0 0.0 0 0 0)
                  (bind _open_close (Timeline|Open/Close Play)
                    (:Update
                      (Transformation|SetRelativeRotation _door (Math|Rotator|MakeRotator 0.0 0.0 _open_close) false false)
                      (bind _asthird_person_character_2 (Utilities|Casting|CastToThirdPersonCharacter (Game|Player|GetPlayerPawn 0)))
                      (bind _isa (Utilities|FlowControl|FlipFlop)
                        (:A
                          _)
                        (:B
                          _))
                      (Pawn|Input|AddMovementInput _asthird_person_character_2 "1.000000,0.000000, 0" (Math|Float|SelectFloat 0.01 -0.01 _isa) false)
                      (Utilities|Array|RemoveItem (Variables|Actor|GetTags) "Door"))))))))))))

(fn ConstructionScript)