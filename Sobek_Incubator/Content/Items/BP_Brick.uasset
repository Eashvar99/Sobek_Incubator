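; Physics brick prop that plays surface-specific impact sounds and can return to its starting placement.
; Hard hits on any axis pick a cue from the physical surface type, with a DoOnce and short delay throttling repeats.
; Shortly after BeginPlay it saves its transform and binds to the player pause menu's reset dispatch, which zeroes velocity and restores that transform.
; Disconnected scene-capture post-process code never runs.
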(event Custom|Reset
  (Physics|SetPhysicsLinearVelocity (Variables|Default|GetStaticMesh) "0, 0, 0" false "None")
  (Transformation|SetWorldTransform (Variables|Default|GetStaticMesh) (Variables|Default|GetLocation) false false))

(event Collision|EventHit
  (params (MyComp :type Primitive%20Component%20Object%20Reference) (Other :type Actor%20Object%20Reference) (OtherComp :type Primitive%20Component%20Object%20Reference) (bSelfMoved :type Boolean) (HitLocation :type Vector :default "0, 0, 0") (HitNormal :type Vector :default "0, 0, 0") (NormalImpulse :type Vector :default "0, 0, 0") (Hit :type Hit%20Result%20Structure%20%28by%20ref%29))
  (if (Math|Boolean|ORBoolean (> (.x NormalImpulse) 7e+02) (> (.y NormalImpulse) 7e+02) (> (.z NormalImpulse) 7e+02) (< (.x NormalImpulse) -7e+02) (< (.y NormalImpulse) -7e+02) (< (.z NormalImpulse) -7e+02))
    (Utilities|FlowControl|DoOnce false :!label _label
      (:Completed
        (switch Utilities|FlowControl|Switch|SwitchonEPhysicalSurface (Collision|GetSurfaceType Hit)
          (:SurfaceType_Default
            _)
          (:SurfaceType1
            (Audio|PlaySoundatLocation "/Game/Sound/WoodHit_Cue.WoodHit_Cue" HitLocation "0, 0, 0" 1.0 1.0 0.0 0 0 0 :!label _label_2))
          (:SurfaceType2
            (Audio|PlaySoundatLocation "/Game/Sound/GrassHit_Cue.GrassHit_Cue" HitLocation "0, 0, 0" 1.0 1.0 0.0 0 0 0 :!label _label_3))
          (:SurfaceType3
            (Audio|PlaySoundatLocation "/Game/Sound/StoneHit_Cue.StoneHit_Cue" HitLocation "0, 0, 0" 1.0 1.0 0.0 0 0 0 :!label _label_4))
          (:SurfaceType4
            (goto _label_4))
          (:SurfaceType5
            (Audio|PlaySoundatLocation "/Game/Sound/GlassHit_Cue.GlassHit_Cue" HitLocation "0, 0, 0" 1.0 1.0 0.0 0 0 0))
          (:SurfaceType6
            (goto _label_3))
          (:SurfaceType7
            (Audio|PlaySoundatLocation "/Game/Sound/MetalHit_Cue.MetalHit_Cue" HitLocation "0, 0, 0" 1.0 1.0 0.0 0 0 0))
          (:SurfaceType8
            _)
          (:SurfaceType9
            (goto _label_2))
          (:SurfaceType10
            (goto _label_4))
          (:SurfaceType11
            (Audio|PlaySoundatLocation "/Game/Sound/GateHit_Cue.GateHit_Cue" HitLocation "0, 0, 0" 0.5 1.0 0.0 0 0 0)))
        (Utilities|FlowControl|Delay 0.1)
        (goto _label Reset)))))

(event EventBeginPlay
  (Utilities|FlowControl|Delay 0.2)
  (Variables|Default|SetLocation (Transformation|GetWorldTransform (Variables|Default|GetStaticMesh)))
  (bind _asthird_person_character (Utilities|Casting|CastToThirdPersonCharacter (Game|Player|GetPlayerPawn 0)))
  (EventDispatchers|BindEventtoResetDispatch (Variables|/Game/_StarterContent/ThirdPersonBP/Blueprints/ThirdPersonCharacter.ThirdPersonCharacter_C|GetPauseMenu _asthird_person_character) (delegate Custom|Reset)))

(event EventTick
  (params (DeltaSeconds :type Float%20%28single-precision%29)))

(fn ConstructionScript)